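; BP_GuideActor is a guide actor in OceanVillage that moves toward targets using homing projectile movement.
; Its movement is deactivated on BeginPlay and toggled by IsMove, which also forwards the state to the parent implementation.
; SetHoming assigns a valid component as the homing target.
; An event that picks a random tagged BP_TargetPoint through the texture fish character remains, but its looping timer setup is disconnected and never runs.
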(event Custom|EventMoveToTarget
  (bind _outactors (Actor|GetAllActorsOfClasswithTag "/Game/Dev/BP/OceanVillage/Actors/BP_TargetPoint.BP_TargetPoint_C" "Random"))
  (bind _returnvalue (Class|TextureFishCharacter|RandomPoint (Variables|Default|GetCBP_TextureFishRef) _outactors))
  (bind _asbp_target_point (Utilities|Casting|CastToBP_TargetPoint _returnvalue))
  (Variables|/Script/Engine.ProjectileMovementComponent|SetHomingTargetComponent (Variables|Default|GetProjectileMovement) (Variables|/Script/Engine.Actor|GetRootComponent _asbp_target_point)))

(event EventBeginPlay
  (Components|Activation|Deactivate (Variables|Default|GetProjectileMovement)))

(event EventIsMove
  (params (isStart :type Boolean))
  (if isStart
    (Components|Activation|Activate (Variables|Default|GetProjectileMovement) true)
    (else
      (Components|Activation|Deactivate (Variables|Default|GetProjectileMovement))))
  (|CallParentFunction isStart))

(event EventSetHoming
  (params (_targetPoint :type Scene%20Component%20Object%20Reference))
  (Utilities|IsValid _targetPoint
    (:Is%20Valid
      (Variables|/Script/Engine.ProjectileMovementComponent|SetHomingTargetComponent (Variables|Default|GetProjectileMovement) _targetPoint))))

(fn ConstructionScript)