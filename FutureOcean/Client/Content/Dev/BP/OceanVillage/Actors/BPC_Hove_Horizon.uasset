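; Actor component that makes its owning actor bob horizontally along the world Y axis.
; BeginPlay caches the owner's starting location, then Tick accumulates time and sets the owner's position to that origin plus a sine offset on Y.
; HoverSpeed sets the frequency and HoverHeight the sideways amplitude, while X and Z stay locked to their starting values.
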(event EventBeginPlay
  (Variables|Default|SetActorStopLocation (Transformation|GetActorLocation (Components|GetOwner))))

(event EventTick
  (params (DeltaSeconds :type Float%20%28single-precision%29))
  (bind _actorstoplocation (Variables|Default|GetActorStopLocation))
  (bind _output_get (Variables|Default|SetTime (+ (Variables|Default|GetTime) (Utilities|Time|GetWorldDeltaSeconds))))
  (Transformation|SetActorLocation (Components|GetOwner) (Math|Vector|MakeVector (.x _actorstoplocation) (+ (.y _actorstoplocation) (* (Math|Trig|Sin(Radians) (* _output_get (Variables|Default|GetHoverSpeed))) (Variables|Default|GetHoverHeight))) (.z _actorstoplocation)) false false))