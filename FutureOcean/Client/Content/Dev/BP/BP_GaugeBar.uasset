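; BP_GaugeBar is a world-space progress gauge that can be swapped for a fish name plate.
; SetGaugeValue drives the Progress parameter on the plane's dynamic material; the construction script picks the Camo or Lumi gauge material by level name.
; AddFishName hides the gauge and shows a rescaled name plane with the supplied material.
; Tick orients the actor along the direction from the NDisplay_MainWall actor to itself.
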(event Custom|SetGaugeValue
  (params (ProgressValue :type Float%20%28double-precision%29))
  (bind _output_get (Variables|Default|SetValue ProgressValue))
  (Rendering|Material|SetScalarParameterValue (Variables|Default|GetMID_Plane) "Progress" _output_get :!class /Script/Engine.MaterialInstanceDynamic))

(event EventBeginPlay
  (bind _returnvalue (Actor|GetActorOfClass "/Game/nDisplay/nDisplay_MainWall.nDisplay_MainWall_C"))
  (Variables|Default|SetnDisplay _returnvalue)
  (bind _returnvalue_2 (Rendering|Material|CreateDynamicMaterialInstance (Variables|Default|GetPlane) 0 0 "None" :!class /Script/Engine.PrimitiveComponent))
  (Variables|Default|SetMID_Plane _returnvalue_2)
  (Rendering|SetVisibility (Variables|Default|GetFishNamePlane) false false)
  (Rendering|SetVisibility (Variables|Default|GetPlane) true false))

(event EventTick
  (params (DeltaSeconds :type Float%20%28single-precision%29))
  (Transformation|SetActorRotation (Math|Rotator|FindLookatRotation (Transformation|GetActorLocation (Variables|Default|GetnDisplay)) (Transformation|GetActorLocation))))

(fn ConstructionScript
  (Rendering|Material|SetScalarParameterValueonMaterials (Variables|Default|GetPlane) "Progress" (Variables|Default|GetValue))
  (bind _returnvalue (Game|GetCurrentLevelName true))
  (if (Utilities|Enum|Equal(Enum) _returnvalue "CamouFlageFish_Wall_Dev")
    (Rendering|Material|SetMaterial (Variables|Default|GetPlane) 0 "/Game/GaugeTest/MI_Camo_Gauge.MI_Camo_Gauge")
    (else
      (Rendering|Material|SetMaterial (Variables|Default|GetPlane) 0 "/Game/GaugeTest/MI_Lumi_Gauge.MI_Lumi_Gauge"))))

(fn AddFishName
  (params (M_FishName :type Material%20Interface%20Object%20Reference) (NewScale3D :type Vector :default "1.000000,0.500000,1.000000"))
  (Utilities|FlowControl|Sequence
    (:then_0
      (Rendering|Material|SetMaterial (Variables|Default|GetFishNamePlane) 0 M_FishName)
      (Rendering|SetVisibility (Variables|Default|GetPlane) false false)
      (Rendering|SetVisibility (Variables|Default|GetFishNamePlane) true false))
    (:then_1
      (CallFunction|SetLocalScaleFishNamePlane NewScale3D))))

(fn SetLocalLocationFishNamePlane
  (params (DeltaLocation :type Vector))
  (Transformation|AddLocalOffset (Variables|Default|GetFishNamePlane) DeltaLocation false false))

(fn SetLocalScaleFishNamePlane
  (params (NewScale3D :type Vector :default "1.000000,0.500000,1.000000"))
  (Transformation|SetRelativeScale3D (Variables|Default|GetFishNamePlane) NewScale3D))