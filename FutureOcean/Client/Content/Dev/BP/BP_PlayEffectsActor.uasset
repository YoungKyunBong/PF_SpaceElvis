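; BP_PlayEffectsActor is a timed step that plays a set of Niagara effects, then hands control back to a manager.
; Its MyStep event waits for a start delay, then activates the Niagara component on every actor in NiagaraActors with a reset.
; After a second delay it deactivates them all and calls NextStep on the Manager passed into the event.
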(event EventMyStep
  (params (Manager :type Step%20Manager%20Object%20Reference))
  (Utilities|FlowControl|Delay (Variables|Default|GetDuration_EffectPlay))
  (for _array_element (Variables|Default|GetNiagaraActors)
    (Components|Activation|SetActive (Variables|/Script/Niagara.NiagaraActor|GetNiagaraComponent _array_element) true true))
  (Utilities|FlowControl|Delay (Variables|Default|GetDuration_EffectEnd))
  (for _array_element_2 (Variables|Default|GetNiagaraActors)
    (Components|Activation|SetActive (Variables|/Script/Niagara.NiagaraActor|GetNiagaraComponent _array_element_2) false true))
  (Class|StepManager|NextStep Manager))

(fn ConstructionScript)