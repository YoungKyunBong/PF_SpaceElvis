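; BP_BGTrashActor is a trash actor in the CleaningOcean game that bobs vertically and can dissolve away.
; On BeginPlay it stores its location, creates a dynamic material on its mesh and starts a timeline that drives a sine-wave hover from accumulated time.
; DissolveTrashEvent plays a second timeline that animates the material's Dissolve parameter and sets IsPlayTrash when finished.
; The construction script and DissolveFunction are empty.
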(event Custom|VerticalMoveEvent
  (bind _verticalmovet (Variables|Default|GetVerticalMoveT))
  (Components|Timeline|SetPlayRate _verticalmovet (/ 1.0 (Variables|Default|GetTimetoSeconds%28insec%29)))
  (Components|Timeline|PlayfromStart _verticalmovet))

(event Custom|DissolveTrashEvent
  (Components|Timeline|PlayfromStart (Variables|Default|GetDissolveTrashT)))

(event EventBeginPlay
  (Variables|Default|SetActorStopLocation (Transformation|GetActorLocation))
  (CallFunction|VerticalMoveEvent)
  (bind _returnvalue (Rendering|Material|CreateDynamicMaterialInstance (Variables|Default|GetStaticMesh) 0 0 "None" :!class /Script/Engine.PrimitiveComponent))
  (Variables|Default|SetDyMaterial_Trashs _returnvalue))

(fn ConstructionScript)

(fn DissolveFunction)