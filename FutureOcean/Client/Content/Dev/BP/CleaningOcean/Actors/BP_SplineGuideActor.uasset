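; Guide actor that travels along a BP_SplinePath spline for the CleaningOcean whale and the LuminaryFish level.
; Two timelines set its transform by spline distance, with play rates derived from travel durations.
; MoveObjectT's first finish picks a Left or Right tagged path from the whale's side; later finishes notify the whale.
; Outside CleaningOcean_Wall_Dev, LuminaryFishMoveT starts on BeginPlay and loops, with events pausing or resuming it by the fish's ray-hit state.
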(event Custom|EndPath)

(event Custom|TimeLineStop
  (Audio|Components|Audio|Stop (Variables|Default|GetMoveObjectT)))

(event Custom|TimeLinePlay
  (Audio|Components|Audio|Play (Variables|Default|GetMoveObjectT)))

(event Custom|RayHitStop
  ;[1 1 1] Ray Hit
  (if (not (Variables|/Game/Dev/BP/CamouFlageFish/Actors/CBP_P_CamouFish.CBP_P_CamouFish_C|GetIsRayHit (Variables|Default|GetBP_LuminaryFish)))
    (Audio|Components|Audio|Stop (Variables|Default|GetLuminaryFishMoveT))))

(event Custom|RayOutPlay
  ;[1 1 1] Ray Hit
  (if (Variables|/Game/Dev/BP/CamouFlageFish/Actors/CBP_P_CamouFish.CBP_P_CamouFish_C|GetIsRayHit (Variables|Default|GetBP_LuminaryFish))
    (Audio|Components|Audio|Play (Variables|Default|GetLuminaryFishMoveT))))

(event Custom|ClearPlay
  ;[1 1 1] Ray Hit
  (Audio|Components|Audio|Play (Variables|Default|GetLuminaryFishMoveT)))

(event EventBeginPlay
  (Components|Timeline|SetPlayRate (Variables|Default|GetMoveObjectT) (/ 1.0 (Variables|Default|GetTimeToComponent%28in%20Sec%29)))
  (bind _returnvalue (Game|GetCurrentLevelName true))
  (if (not (Utilities|Enum|Equal(Enum) _returnvalue "CleaningOcean_Wall_Dev"))
    (bind _returnvalue_2 (Game|GetCurrentLevelName true))
    (if (Utilities|Enum|Equal(Enum) _returnvalue_2 "LuminaryFish_Wall_Dev")
      _
      (else
        _))
    (Components|Timeline|SetPlayRate (Variables|Default|GetLuminaryFishMoveT) (/ 1.0 (Variables|Default|GetTimeToLuminaryFish%28insec%29)))
    (Components|Timeline|PlayfromStart (Variables|Default|GetLuminaryFishMoveT))))

(fn ConstructionScript)

(fn SelectSideType
  (bind _output_get (Variables|Default|SetSideType (Class|WhaleCharacter|GetSideType (Variables|Default|GetBP_WhaleRef))))
  (if (Utilities|Enum|Equal(Enum) _output_get "LeftSide")
    (bind _outactors (Actor|GetAllActorsOfClasswithTag "/Game/Dev/BP/CleaningOcean/Actors/BP_SplinePath.BP_SplinePath_C" "Left"))
    (for _array_element _outactors
      (Variables|Default|SetSpline%20Ref _array_element)
      (CallFunction|SetRatePlayfromStart 2e+01)
      (Variables|Default|SetbTurn true))
    (else
      (bind _outactors_2 (Actor|GetAllActorsOfClasswithTag "/Game/Dev/BP/CleaningOcean/Actors/BP_SplinePath.BP_SplinePath_C" "Right"))
      (for _array_element_2 _outactors_2
        (Variables|Default|SetSpline%20Ref _array_element_2)
        (CallFunction|SetRatePlayfromStart 15.0)
        (Variables|Default|SetbTurn true)))))

(fn SetRatePlayfromStart
  (params (TimeToComponent :type Float%20%28double-precision%29))
  (bind _moveobjectt (Variables|Default|GetMoveObjectT))
  (Variables|Default|SetTimeToComponent%28in%20Sec%29 TimeToComponent)
  (Components|Timeline|SetPlayRate _moveobjectt (/ 1.0 (Variables|Default|GetTimeToComponent%28in%20Sec%29)))
  (Components|Timeline|PlayfromStart _moveobjectt))