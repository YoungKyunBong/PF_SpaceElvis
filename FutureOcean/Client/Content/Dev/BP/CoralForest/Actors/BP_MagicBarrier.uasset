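; BP_MagicBarrier is a coral forest actor that sends a Niagara fish effect (NSFish) swimming toward a target point.
; BeginPlay assigns the effect asset; Activate_FishSwim activates it and the projectile movement, homing on TargetPoint.
; A sphere overlap plays a timeline that lerps max speed and homing acceleration toward a low fixed value.
; Each lerp starts from the other property's live value, re-read every update.
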(event OnComponentBeginOverlap(Sphere)
  (params (OverlappedComponent :type Primitive%20Component%20Object%20Reference) (OtherActor :type Actor%20Object%20Reference) (OtherComp :type Primitive%20Component%20Object%20Reference) (OtherBodyIndex :type Integer) (bFromSweep :type Boolean) (SweepResult :type Hit%20Result%20Structure%20%28by%20ref%29))
  (bind _projectilemovement (Variables|Default|GetProjectileMovement))
  (bind _projectilemovement_2 (Variables|Default|GetProjectileMovement))
  (bind _float (Timeline|MovementSpeedT Play)
    (:Update
      (Variables|/Script/Engine.ProjectileMovementComponent|SetMaxSpeed _projectilemovement (Math|Float|Lerp (Variables|/Script/Engine.ProjectileMovementComponent|GetHomingAccelerationMagnitude _projectilemovement_2) 5e+01 _float))
      (Variables|/Script/Engine.ProjectileMovementComponent|SetHomingAccelerationMagnitude _projectilemovement (Math|Float|Lerp (Class|MovementComponent|GetMaxSpeed _projectilemovement_2) 5e+01 _float)))))

(event Custom|Activate_FishSwim
  (Components|Activation|Activate (Variables|Default|GetNS_Fish) false)
  (Components|Activation|Activate (Variables|Default|GetProjectileMovement) false)
  (Variables|/Script/Engine.ProjectileMovementComponent|SetHomingTargetComponent (Variables|Default|GetProjectileMovement) (Variables|/Script/Engine.Actor|GetRootComponent (Variables|Default|GetTargetPoint))))

(event EventBeginPlay
  (Class|NiagaraComponent|SetAsset (Variables|Default|GetNS_Fish) (Variables|Default|GetNS_FishAsset) true))

(fn ConstructionScript)