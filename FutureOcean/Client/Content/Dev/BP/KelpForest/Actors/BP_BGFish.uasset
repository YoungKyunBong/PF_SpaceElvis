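; BP_BGFish is a background fish actor for the KelpForest level that travels along a referenced spline.
; A looping timeline maps its MoveTrack value to distance along the spline, setting the actor's world location and rotation to match.
; BeginPlay sets the timeline play rate from TimetoComponentInSec as the travel duration.
; A Play event reapplies that rate and restarts the timeline from the start.
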(event Custom|Play
  (Components|Timeline|SetPlayRate (Variables|Default|Get타임라인) (/ 1.0 (Variables|Default|GetTimeto%20Component%28In%20Sec%29)))
  (Components|Timeline|PlayfromStart (Variables|Default|Get타임라인)))

(event EventBeginPlay
  (Components|Timeline|SetPlayRate (Variables|Default|Get타임라인) (/ 1.0 (Variables|Default|GetTimeto%20Component%28In%20Sec%29))))

(fn ConstructionScript)