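; BP_ChangePlayMeshActor is a step actor that switches the look and visibility of two referenced static mesh actors when its step runs.
; MyStep applies an enable material to one mesh and shows it, then applies a disable material to the other and hides it only outside VR.
; It then calls NextStep on the passed Manager to advance the sequence.
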(event EventBeginPlay)

(event Collision|EventActorBeginOverlap
  (params (OtherActor :type Actor%20Object%20Reference)))

(event EventTick
  (params (DeltaSeconds :type Float%20%28single-precision%29)))

(event EventMyStep
  (params (Manager :type Step%20Manager%20Object%20Reference))
  (bind _disablemeshactor (Variables|Default|GetDisableMeshActor))
  (bind _enablemeshactor (Variables|Default|GetEnableMeshActor))
  (bind _staticmeshcomponent (Variables|/Script/Engine.StaticMeshActor|GetStaticMeshComponent _disablemeshactor))
  (bind _staticmeshcomponent_2 (Variables|/Script/Engine.StaticMeshActor|GetStaticMeshComponent _enablemeshactor))
  (Utilities|FlowControl|Sequence
    (:then_0
      (Rendering|Material|SetMaterial _staticmeshcomponent_2 0 (Variables|Default|GetEnableMaterial_Inst))
      (Rendering|SetVisibility _staticmeshcomponent_2 true false))
    (:then_1
      (Rendering|Material|SetMaterial _staticmeshcomponent 0 (Variables|Default|GetDisableMaterial_Inst))
      (if (not (Variables|Default|GetIsVR))
        (Rendering|SetVisibility _staticmeshcomponent false false)))
    (:then_2
      (Class|DefaultManager|NextStep Manager))))

(fn ConstructionScript)