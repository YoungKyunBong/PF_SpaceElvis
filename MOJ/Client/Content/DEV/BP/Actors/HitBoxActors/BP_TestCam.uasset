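; BP_TestCam is a test actor that detects which tagged actor its arrow component is pointing at.
; Every tick it runs a long, debug-drawn line trace along the arrow and reads the hit actor's first tag.
; It caches that tag in HitNumber and prints only on a change, showing a Korean "please focus on the screen" warning when the trace stops hitting anything.
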(event EventTick
  (params (DeltaSeconds :type Float%20%28single-precision%29))
  (bind _arrow (Variables|Default|GetArrow))
  (bind _returnvalue (Transformation|GetWorldLocation _arrow))
  (bind (_outhit _returnvalue_2) (Collision|LineTraceByChannel _returnvalue (+ (* (Math|Vector|GetForwardVector _arrow) 1e+05) _returnvalue) "TraceTypeQuery3" false 0 "ForOneFrame"))
  (if _returnvalue_2
    ;[1 1 1] Hit
    (if (not (== (Variables|Default|GetHitNumber) (Utilities|Array|Get(acopy) (Variables|/Script/Engine.Actor|GetTags (.HitActor (Collision|BreakHitResult _outhit))))))
      (bind _output_get (Variables|Default|SetHitNumber (Utilities|Array|Get(acopy) (Variables|/Script/Engine.Actor|GetTags (.HitActor (Collision|BreakHitResult _outhit))))))
      (Development|PrintString (Utilities|String|ToString(Name) _output_get)))
    (else
      ;[1 1 1] NoHit
      (if (not (== (Variables|Default|GetHitNumber) "None"))
        (Variables|Default|SetHitNumber "None")
        (Development|PrintString "@@화면에 집중해주세요@@ 
@@화면에 집중해주세요@@ 
@@화면에 집중해주세요@@ 
@@화면에 집중해주세요@@ 
@@화면에 집중해주세요@@")))))

(fn ConstructionScript)