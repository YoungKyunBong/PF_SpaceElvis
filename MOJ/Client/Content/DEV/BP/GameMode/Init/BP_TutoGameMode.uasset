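; Tutorial game mode that plays a tutorial video for a VR pawn, driven by remote CMS controller events from the Game Manager.
; The start event opens the media source, then playback and a timeline-driven pawn fade begin once media opens.
; Play and stop events resume or pause the video once started.
; When the video ends, it notifies the Game Manager, closes the player and opens the manager's named level after a short delay.
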(event Custom|RecvCmsControllerStart_이벤트
  (CallFunction|RecvOpenLevel))

(event Custom|EndTuto
  (Class|GameManager|SendTutoEnd (CallFunction|GetGameManager))
  (Media|MediaPlayer|Close (Variables|Default|GetNewVar) :!class /Script/MediaAssets.MediaPlayer)
  (Utilities|FlowControl|Delay 0.2)
  (Game|OpenLevel(byName) (Utilities|String|StringToName (Variables|/Script/MojMovieClient.GameManager|GetLevelName (CallFunction|GetGameManager)))))

(event Custom|RecvOpenLevel
  (Variables|Default|SetIsMovieStart true)
  (Media|MediaPlayer|OpenSource (Variables|Default|GetNewVar) (Variables|Default|GetNewVar_0))
  (EventDispatchers|AssignOnMediaOpened (Variables|Default|GetNewVar) (delegate Custom|OnMediaOpened_이벤트)))

(event Custom|PauseMovie
  (if (Variables|Default|GetIsMovieStart)
    (Sequencer|Player|Pause (Variables|Default|GetNewVar))))

(event Custom|OnMediaOpened_이벤트
  (params (OpenedUrl :type String))
  (Media|MediaPlayer|Play (Variables|Default|GetNewVar) :!class /Script/MediaAssets.MediaPlayer)
  (Media|MediaPlayer|BindEventtoOnEndReached (Variables|Default|GetNewVar) (delegate Custom|EndTuto))
  (bind _새_트랙_0 (Timeline|타임라인 Play)
    (:Update
      (Default|SetFade (Variables|Default|GetPawn) _새_트랙_0))))

(event Custom|RecvCmsControllerPlayInBP_이벤트
  (CallFunction|PlayMovie))

(event Custom|RecvCmsControllerStopInBP_이벤트
  (CallFunction|PauseMovie))

(event Custom|PlayMovie
  (if (Variables|Default|GetIsMovieStart)
    (Media|MediaPlayer|Play (Variables|Default|GetNewVar) :!class /Script/MediaAssets.MediaPlayer)))

(event EventBeginPlay
  (bind _returnvalue (Actor|GetActorOfClass "/Game/VRTemplate/Blueprints/VRPawn.VRPawn_C"))
  (Variables|Default|SetPawn _returnvalue)
  (Media|MediaPlayer|Close (Variables|Default|GetNewVar) :!class /Script/MediaAssets.MediaPlayer)
  (EventDispatchers|AssignRecvCmsControllerStart (CallFunction|GetGameManager) (delegate Custom|RecvCmsControllerStart_이벤트))
  (EventDispatchers|AssignRecvCmsControllerPlayinBP (CallFunction|GetGameManager) (delegate Custom|RecvCmsControllerPlayInBP_이벤트))
  (EventDispatchers|AssignRecvCmsControllerStopinBP (CallFunction|GetGameManager) (delegate Custom|RecvCmsControllerStopInBP_이벤트)))

(fn ConstructionScript)