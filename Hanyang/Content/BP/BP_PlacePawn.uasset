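; BP_PlacePawn is a walking, mouse-look player pawn with a toggleable cursor.
; On BeginPlay it applies capsule size and max step height from variables to the capsule and CharacterMovement.
; Axis inputs move it along actor forward and right, yaw the actor, and pitch the camera within about ±89 degrees.
; A FlipFlop, fired by SetMouseCursor or FlipFlopInit, alternates between visible-cursor Game-and-UI and hidden-cursor Game-Only input.
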(event Custom|FlipFlopInit
  (bind _returnvalue (Game|GetPlayerController 0))
  (bind _returnvalue_2 (Game|GetPlayerController 0))
  (Utilities|FlowControl|FlipFlop
    (:A
      (Variables|/Script/Engine.PlayerController|SetbShowMouseCursor _returnvalue true)
      (Input|SetInputModeGameandUI _returnvalue 0 "LockAlways" true false))
    (:B
      (Variables|/Script/Engine.PlayerController|SetbShowMouseCursor _returnvalue_2 false)
      (Input|SetInputModeGameOnly _returnvalue_2 false))))

(event EventBeginPlay
  (Components|Capsule|SetCapsuleSize (Variables|Collision|GetCapsuleComponent) (Variables|Default|GetIn%20Radius) (Variables|Default|GetIn%20Half%20Height) true)
  (Variables|/Script/Engine.CharacterMovementComponent|SetMaxStepHeight (Variables|Character|GetCharacterMovement) (Variables|Default|Get최대%20스텝%20높이)))

(event Input|ActionEvents|InputActionSetMouseCursor
  (params (Key :type Key%20Structure :default "None"))
  (bind _returnvalue (Game|GetPlayerController 0))
  (bind _returnvalue_2 (Game|GetPlayerController 0))
  (:Pressed
    (Utilities|FlowControl|FlipFlop
      (:A
        (Variables|/Script/Engine.PlayerController|SetbShowMouseCursor _returnvalue true)
        (Input|SetInputModeGameandUI _returnvalue 0 "LockAlways" true false))
      (:B
        (Variables|/Script/Engine.PlayerController|SetbShowMouseCursor _returnvalue_2 false)
        (Input|SetInputModeGameOnly _returnvalue_2 false)))))

(event Input|AxisEvents|InputAxisMoveRight
  (params (AxisValue :type Float%20%28single-precision%29))
  (Pawn|Input|AddMovementInput (* AxisValue (Transformation|GetActorRightVector)) 1.0 false))

(event Input|AxisEvents|InputAxisMouseX
  (params (AxisValue :type Float%20%28single-precision%29))
  (Class|Actor|AddActorWorldRotation (Math|Rotator|MakeRotator 0.0 0.0 AxisValue)))

(event Input|AxisEvents|InputAxisMouseY
  (params (AxisValue :type Float%20%28single-precision%29))
  (bind _camera (Variables|Default|GetCamera))
  (bind _camera_2 (Variables|Default|GetCamera))
  (bind _relativerotation (Variables|/Script/Engine.SceneComponent|GetRelativeRotation _camera_2))
  (bind _pitch (Math|Rotator|BreakRotator _relativerotation))
  (if (Math|Float|InRange(Float) _pitch -89.0 89.0)
    (Transformation|AddRelativeRotation (Variables|Default|GetCamera) (Math|Rotator|MakeRotator 0.0 AxisValue 0.0) false false)
    (else
      (Utilities|FlowControl|Sequence
        (:then_0
          (if (Math|Float|NearlyEqual(Float) _pitch 89.0 1.0)
            (Transformation|SetRelativeRotation _camera "89.000000,0.000000,0.000000" false false)))
        (:then_1
          (if (Math|Float|NearlyEqual(Float) _pitch -89.0 1.0)
            (Transformation|SetRelativeRotation _camera "-89.000000,0.000000,0.000000" false false)))))))

(event Input|AxisEvents|InputAxisMoveForward
  (params (AxisValue :type Float%20%28single-precision%29))
  (Pawn|Input|AddMovementInput (* AxisValue (Transformation|GetActorForwardVector)) 1.0 false))

(fn ConstructionScript)